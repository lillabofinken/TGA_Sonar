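; Spinning active sonar actor that sweeps a scene capture through a full circle and builds a sonar display image.
; Each tick it derives yaw from game time and RotationSpeed, rotates SonarCapture, and writes angle and half-FOV to MPC_PanoramaStitch.
; M_PanoramaStitch then draws into RT_SonarPanorama, which a compute shader turns into RT_SonarDisplay using the current angle, half-FOV and Range.
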(event `self.ReceiveBeginPlay`)

(event `self.ReceiveTick`
  (params (DeltaSeconds :type "Float (single-precision)"))
  (bind _returnvalue (/ (`SonarCaptureComponent.HorizontalCustomFOVAngle` (`self.SonarCapture`)) 2.0))
  (bind _returnvalue_2 (* (`KismetMathLibrary.Fraction` (/ (`KismetSystemLibrary.GetGameTimeInSeconds`) (`self.RotationSpeed`))) 360.0))
  (`self.RotateCaptures` _returnvalue_2)
  (`KismetMaterialLibrary.SetScalarParameterValue` "/Game/ActiveSonar/MPC_PanoramaStitch.MPC_PanoramaStitch" "Rotation" _returnvalue_2)
  (`KismetMaterialLibrary.SetScalarParameterValue` "/Game/ActiveSonar/MPC_PanoramaStitch.MPC_PanoramaStitch" "Fov" _returnvalue)
  (`KismetRenderingLibrary.DrawMaterialToRenderTarget` "/Game/ActiveSonar/RT_SonarPanorama.RT_SonarPanorama" "/Game/ActiveSonar/M_PanoramaStitch.M_PanoramaStitch")
  (`DeformationCSLibrary.ExecuteRTComputeShader` "/Game/ActiveSonar/RT_SonarDisplay.RT_SonarDisplay" "/Game/ActiveSonar/RT_SonarPanorama.RT_SonarPanorama" _returnvalue_2 _returnvalue (`self.Range`)))

(event `RotateCaptures`
  (params (Rotation :type "Float (double-precision)"))
  (bind (_returnvalue_roll _returnvalue_pitch) (`KismetMathLibrary.BreakRotator` (`SceneComponent.K2_GetComponentRotation` (`self.SonarCapture`))))
  (`SceneComponent.K2_SetRelativeRotation` (`self.SonarCapture`) (`KismetMathLibrary.MakeRotator` _returnvalue_roll _returnvalue_pitch Rotation) false false))

(fn `UserConstructionScript`)