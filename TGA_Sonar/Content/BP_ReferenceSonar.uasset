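; BP_ReferenceSonar is an actor that takes a one-time sonar-style depth scan of its surroundings on BeginPlay.
; It sweeps a ResX by ResY grid of Visibility line traces around the full horizontal circle and through a 45-degree vertical arc.
; Normalized hit distances become grayscale colors, written into the Temp_Blod texture through UpdateTexturePixels.
; A random one-eighth or so of the rays are debug-drawn.
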(event `self.ReceiveTick`
  (params (DeltaSeconds :type "Float (single-precision)")))

(event `self.ReceiveActorBeginOverlap`
  (params (OtherActor :type "Actor Object Reference")))

(event `self.ReceiveBeginPlay`
  (bind _returnvalue (`self.K2_GetActorLocation`))
  (`KismetArrayLibrary.Array_Clear` (`self.Distances`))
  (for _index (range (`self.ResX`))
    (for _index_2 (range (`self.ResY`))
      (if (`KismetMathLibrary.RandomBoolWithWeight` 0.125)
        (bind _returnvalue_2 (+ _returnvalue (* (`KismetMathLibrary.RotateAngleAxis` (`KismetMathLibrary.RotateAngleAxis` (`self.GetActorForwardVector`) (* _index_2 (/ 45.0 (`self.ResY`)) 1.0) (`self.GetActorRightVector`)) (* _index (/ 360.0 (`self.ResX`)) 1.0) (0.0 0.0 1.0)) 1000.0)))
        (bind _outhit (`KismetSystemLibrary.LineTraceSingle` :`Start` _returnvalue :`End` _returnvalue_2 :`TraceChannel` "TraceTypeQuery1" :`DrawDebugType` "ForDuration" :`DrawTime` 10.0))
        (bind _returnvalue_3 (/ (`.Distance` (`GameplayStatics.BreakHitResult` _outhit)) 1000.0))
        (`KismetArrayLibrary.Array_Add` (`self.Distances`) (`KismetMathLibrary.Conv_LinearColorToColor` (`KismetMathLibrary.MakeColor` _returnvalue_3 _returnvalue_3 _returnvalue_3)))
        (else
          (bind _outhit_2 (`KismetSystemLibrary.LineTraceSingle` :`Start` _returnvalue :`End` _returnvalue_2 :`TraceChannel` "TraceTypeQuery1" :`TraceColor` (struct :`B` 1.0 :`A` 1.0) :`DrawTime` 1.0))
          (bind _returnvalue_4 (/ (`.Distance` (`GameplayStatics.BreakHitResult` _outhit_2)) 1000.0))
          (`KismetArrayLibrary.Array_Add` (`self.Distances`) (`KismetMathLibrary.Conv_LinearColorToColor` (`KismetMathLibrary.MakeColor` _returnvalue_4 _returnvalue_4 _returnvalue_4)))))))
  (`SonarFunctionLibrary.UpdateTexturePixels` "/Game/Temp_Blod.Temp_Blod" (`self.Distances`) (`self.ResX`) (`self.ResY`)))

(fn `UserConstructionScript`)