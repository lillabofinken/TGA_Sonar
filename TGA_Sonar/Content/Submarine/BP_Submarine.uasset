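; Player-controlled submarine with physics-driven movement and a camera that switches between its map, active sonar and passive sonar screens.
; Enhanced Input values feed vertical/forward force and yaw torque in AsyncPhysicsTick, with a speed boost and input-dependent angular damping.
; BeginPlay builds camera transforms facing each screen plus a base view; look and select inputs choose one, and Tick lerps the camera to it.
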(event Custom|LookLerp
  ;[0.5826 0 0] LOOK
  (if (< (Variables|Look|GetLookLerpValuie) 1.0)
    (bind _output_get (Variables|Look|SetLookLerpValuie (Math|Float|Clamp(Float) (+ (Variables|Look|GetLookLerpValuie) (Utilities|Time|GetWorldDeltaSeconds)))))
    (Transformation|SetRelativeTransform (Variables|Default|GetCamera) (Math|Transform|Lerp(Transform) (Transformation|GetRelativeTransform (Variables|Default|GetCamera)) (Variables|Default|GetTargetTransform) _output_get) false false)))

(event Custom|SubmarineMovement
  (bind _returnvalue (Utilities|Time|GetWorldDeltaSeconds))
  (bind _throttlevalue (Variables|Input|GetThrottleValue))
  (bind _speed (Variables|Movement|GetSpeed))
  (bind _sub (Variables|Default|GetSub))
  (bind _sprintinput (Variables|Input|GetSprintInput))
  (bind _returnvalue_2 (* _sprintinput 2e+01))
  (bind _returnvalue_3 (+ _returnvalue_2 1.0))
  (bind _returnvalue_4 (* _throttlevalue _speed _returnvalue "(X=1000000.000000,Y=1000000.000000)" _returnvalue_3))
  ;[1 0 0 0.5] Submarine Control
  (Physics|AddForce (Variables|Default|GetSub) (+ (* (.x _returnvalue_4) (Math|Vector|GetUpVector _sub)) (* (.y _returnvalue_4) (Math|Vector|GetForwardVector _sub))) "None" false))

(event Custom|Steer
  ;[1 0 0 0.5] Submarine Control
  (Class|PrimitiveComponent|AddTorqueinDegrees (Variables|Default|GetSub) (Math|Vector|MakeVector 0.0 0.0 (* (Variables|Input|GetSteerInput) (Utilities|Time|GetWorldDeltaSeconds) (Variables|Movement|GetSteeringSpeed) 5e+08 (+ (* (Variables|Input|GetSprintInput) 1e+01) 1.0))) "None" false))

(event Custom|SetActiveTransform
  (params (Index :type Integer))
  ;[0.5826 0 0] LOOK
  (if (Utilities|Array|IsValidIndex (Variables|Look|GetLookTransforms) Index)
    (Variables|Default|SetTargetTransform (Utilities|Array|Get(acopy) (Variables|Look|GetLookTransforms) Index))
    (else
      (Variables|Default|SetTargetTransform (Variables|Look|GetBaseLookTransform))))
  (Variables|Look|SetRotationIndex Index)
  (Variables|Look|SetLookLerpValuie 0.0))

(event Input|EnhancedActionEvents|EnhancedInputActionIA_Look
  (params (ActionValue :type Float%20%28double-precision%29) (ElapsedSeconds :type Float%20%28double-precision%29) (TriggeredSeconds :type Float%20%28double-precision%29) (InputAction :type Input%20Action%20Object%20Reference :default "/Game/Submarine/IA_Look.IA_Look"))
  (bind _returnvalue (Math|Float|Truncate ActionValue))
  ;[0.5826 0 0] LOOK
  (:Started
    (bind _output_get (Variables|Look|SetRotationIndex (Math|Integer|SelectInt 0 (Math|Integer|SelectInt (- (Utilities|Array|Length (Variables|Look|GetLookTransforms)) 1) (+ (Variables|Look|GetRotationIndex) (Math|Integer|SelectInt (* _returnvalue -1) _returnvalue (== (Variables|Look|GetRotationIndex) 3))) (< (+ (Variables|Look|GetRotationIndex) (Math|Integer|SelectInt (* _returnvalue -1) _returnvalue (== (Variables|Look|GetRotationIndex) 3))) 0)) (> (Math|Integer|SelectInt (- (Utilities|Array|Length (Variables|Look|GetLookTransforms)) 1) (+ (Variables|Look|GetRotationIndex) (Math|Integer|SelectInt (* _returnvalue -1) _returnvalue (== (Variables|Look|GetRotationIndex) 3))) (< (+ (Variables|Look|GetRotationIndex) (Math|Integer|SelectInt (* _returnvalue -1) _returnvalue (== (Variables|Look|GetRotationIndex) 3))) 0)) (- (Utilities|Array|Length (Variables|Look|GetLookTransforms)) 1)))))
    (Variables|Default|SetTargetTransform (Utilities|Array|Get(acopy) (Variables|Look|GetLookTransforms) _output_get))
    (Variables|Look|SetLookLerpValuie 0.0)))

(event Input|EnhancedActionEvents|EnhancedInputActionIA_Steer
  (params (ActionValue :type Float%20%28double-precision%29) (ElapsedSeconds :type Float%20%28double-precision%29) (TriggeredSeconds :type Float%20%28double-precision%29) (InputAction :type Input%20Action%20Object%20Reference :default "/Game/Submarine/IA_Steer.IA_Steer"))
  ;[1 0 0 0.5] Submarine Control
  (:Triggered
    (bind _output_get (Variables|Input|SetSteerInput ActionValue :!label _label))
    (Class|PrimitiveComponent|SetAngularDamping (Variables|Default|GetSub) (Math|Float|SelectFloat 1.0 2.0 (> (Math|Float|Absolute(Float) _output_get) 0.0))))
  (:Canceled
    (goto _label))
  (:Completed
    (goto _label)))

(event Input|EnhancedActionEvents|EnhancedInputActionIA_Throttle
  (params (ActionValue :type Vector%202D%20Structure) (ElapsedSeconds :type Float%20%28double-precision%29) (TriggeredSeconds :type Float%20%28double-precision%29) (InputAction :type Input%20Action%20Object%20Reference :default "/Game/Submarine/IA_Throttle.IA_Throttle"))
  ;[1 0 0 0.5] Submarine Control
  (:Triggered
    (Variables|Input|SetThrottleValue ActionValue :!label _label))
  (:Canceled
    (goto _label))
  (:Completed
    (goto _label)))

(event Input|EnhancedActionEvents|EnhancedInputActionIA_Speed
  (params (ActionValue :type Float%20%28double-precision%29) (ElapsedSeconds :type Float%20%28double-precision%29) (TriggeredSeconds :type Float%20%28double-precision%29) (InputAction :type Input%20Action%20Object%20Reference :default "/Game/Submarine/IA_Speed.IA_Speed"))
  ;[1 0 0 0.5] Submarine Control
  (:Triggered
    (Variables|Input|SetSprintInput ActionValue :!label _label))
  (:Started
    (goto _label))
  (:Canceled
    (goto _label))
  (:Completed
    (goto _label)))

(event Input|EnhancedActionEvents|EnhancedInputActionIA_SelectCam
  (params (ActionValue :type Float%20%28double-precision%29) (ElapsedSeconds :type Float%20%28double-precision%29) (TriggeredSeconds :type Float%20%28double-precision%29) (InputAction :type Input%20Action%20Object%20Reference :default "/Game/Submarine/IA_SelectCam.IA_SelectCam"))
  (bind _returnvalue (Math|Float|Truncate ActionValue))
  ;[0.5826 0 0] LOOK
  (:Started
    (CallFunction|SetActiveTransform _returnvalue)
    (Development|PrintString (Utilities|String|ToString(Integer) _returnvalue))))

(event EventBeginPlay
  (bind _baselooktransform (Variables|Look|GetBaseLookTransform))
  (Utilities|FlowControl|Sequence
    (:then_0
      (Input|AddMappingContext (PlayerController|LocalPlayerSubsystems|GetEnhancedInputLocalPlayerSubsystem (Game|GetPlayerController 0)) "/Game/Submarine/MPC_Submarine.MPC_Submarine" 0 "(bIgnoreAllPressedKeysUntilRelease=True,bForceImmediately=False,bNotifyUserSettings=False)"))
    (:then_1
      (for _array_element (Utilities|Array|MakeArray (Variables|Default|GetSCREEN_Map) (Variables|Default|GetSCREEN_ActiveSonar) (Variables|Default|GetSCREEN_PassiveSonar))
        (Utilities|Array|Add (Variables|Look|GetLookTransforms) (Math|Transform|MakeTransform (+ (* (Math|Vector|GetUpVector _array_element) (Math|Float|MakeLiteralFloat 75.0)) (Variables|/Script/Engine.SceneComponent|GetRelativeLocation _array_element)) (Math|Rotator|FindLookatRotation (+ (* (Math|Vector|GetUpVector _array_element) (Math|Float|MakeLiteralFloat 75.0)) (Variables|/Script/Engine.SceneComponent|GetRelativeLocation _array_element)) (Variables|/Script/Engine.SceneComponent|GetRelativeLocation _array_element)) "1.000000,1.000000,1.000000")))
      (Utilities|Array|Add (Variables|Look|GetLookTransforms) _baselooktransform)
      (Variables|Default|SetTargetTransform _baselooktransform))
    (:then_2)))

(event EventTick
  (params (DeltaSeconds :type Float%20%28single-precision%29))
  (CallFunction|LookLerp))

(event EventAsyncPhysicsTick
  (params (DeltaSeconds :type Float%20%28single-precision%29) (SimSeconds :type Float%20%28single-precision%29))
  (Class|PrimitiveComponent|WakeRigidBody (Variables|Default|GetSub) "None")
  (CallFunction|SubmarineMovement)
  (CallFunction|Steer))

(event Input|MouseEvents|DebugKeyLeftMouseButton
  (params (Key :type Key%20Structure :default "None") (ActionValue :type Input%20Action%20Value%20Structure))
  (:Pressed
    (Transformation|SetRelativeLocation (Variables|Default|GetCamera) "0.000000,0.000000,200.000000" false false)
    (Variables|Look|SetLookLerpValuie 1.0))
  (:Released
    (Variables|Look|SetLookLerpValuie 0.0)))

(fn ConstructionScript)